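; MasterItem is a world item actor, apparently the inventory base, that holds ItemData and exposes getters for name, amount, stackability and image.
; On BeginPlay it passes the image and data to its widget.
; SetItemWorldPopUp spawns or destroys a BP_EquipmentGround pop-up actor, only for a locally controlled player.
; Destruction calls a client remove event that clears the pop-up and still prints debug text; ItemData's RepNotify is empty.
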(event `self.ReceiveBeginPlay`
  (bind _widget (`self.Widget`))
  (message `/Game/Blueprints/Interfaces/Inventory_BPI.SetItemImage` (`WidgetComponent.GetWidget` _widget) (`self.GetItemImage`))
  (message `/Game/Blueprints/Interfaces/Inventory_BPI.SetItemData` (`WidgetComponent.GetWidget` _widget) (`self.ItemData`)))

(event `ShowInfo`
  (params (NewParam :type Boolean) (Owner :type "Actor Object Reference"))
  (bind _popupref (`self.PopUpRef`))
  (if NewParam
    (`/Engine/EditorBlueprintResources/StandardMacros.IsValid` (`self.PopUpRef`)
      (:`Is Not Valid`
        (bind _returnvalue (`|SpawnActorFromClass` "/Game/Blueprints/Inventory/UI/BP_EquipmentGround.BP_EquipmentGround_C" (`self.GetTransform`) "Undefined" "MultiplyWithRoot" Owner (`self.ItemData`) null))
        (set `self.PopUpRef` _returnvalue)))
    (else
      (`/Engine/EditorBlueprintResources/StandardMacros.IsValid` _popupref
        (:`Is Valid`
          (`self.K2_DestroyActor` _popupref))))))

(event `Client_Remove`
  (bind _popupref (`self.PopUpRef`))
  (`KismetSystemLibrary.PrintString` "Hello")
  (`/Engine/EditorBlueprintResources/StandardMacros.IsValid` _popupref
    (:`Is Valid`
      (`self.K2_DestroyActor` _popupref))))

(event `self.ReceiveDestroyed`
  (`self.Client_Remove`))

(event `/Game/Blueprints/Interfaces/Inventory_BPI.SetItemWorldPopUp`
  (params (PopUpState :type Boolean) (OwningPlayer :type "Actor Object Reference"))
  (bind _returnvalue (`self.GetInstigatorController` OwningPlayer))
  (`/Engine/EditorBlueprintResources/StandardMacros.IsValid` _returnvalue
    (:`Is Valid`
      (if (`Controller.IsLocalController` _returnvalue)
        (`self.ShowInfo` PopUpState OwningPlayer)))))

(fn `GetIsStackable`
  (returns (`Is Stackable` :type Boolean))
  (bind (_itemdata_equipmentstats _itemdata_equipementlvl _itemdata_itemrarity _itemdata_averagestatpercentage _itemdata_itemdata) (break `/Game/Blueprints/Inventory/EquipmentItemData` (`self.ItemData`)))
  (return (`.IsStackable_7_7F3981964136D1E5C2B1D0B6A94F1374` (break `/Game/Blueprints/Inventory/ItemData` _itemdata_itemdata))))

(fn `GetItemAmount`
  (returns (NewParam :type Integer))
  (bind (_itemdata_equipmentstats _itemdata_equipementlvl _itemdata_itemrarity _itemdata_averagestatpercentage _itemdata_itemdata) (break `/Game/Blueprints/Inventory/EquipmentItemData` (`self.ItemData`)))
  (return (`.Amount_10_1E37BF4F4EA00B7CB1EC3FB949DD8C1B` (break `/Game/Blueprints/Inventory/ItemData` _itemdata_itemdata))))

(fn `GetItemData`
  (returns (ItemData :type "/Game/Blueprints/Inventory/EquipmentItemData Structure"))
  (return (`self.ItemData`)))

(fn `GetItemImage`
  (returns (`Item Data Item Image` :type "Texture Object Reference"))
  (bind (_itemdata_equipmentstats _itemdata_equipementlvl _itemdata_itemrarity _itemdata_averagestatpercentage _itemdata_itemdata) (break `/Game/Blueprints/Inventory/EquipmentItemData` (`self.ItemData`)))
  (return (`.ItemImage_16_F6D0A68B49ED23E3CCE90597F0C010CB` (break `/Game/Blueprints/Inventory/ItemData` _itemdata_itemdata))))

(fn `GetItemName`
  (returns (`Item Data Name` :type String))
  (bind (_itemdata_equipmentstats _itemdata_equipementlvl _itemdata_itemrarity _itemdata_averagestatpercentage _itemdata_itemdata) (break `/Game/Blueprints/Inventory/EquipmentItemData` (`self.ItemData`)))
  (return (`.Name_8_CC3B75BB4954A3591D2286B204FCF81A` (break `/Game/Blueprints/Inventory/ItemData` _itemdata_itemdata))))

(fn `OnRep_ItemData`)

(fn `UserConstructionScript`)