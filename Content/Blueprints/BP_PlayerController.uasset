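; Player controller Blueprint that manages a targeter actor marking the player's look destination.
; It spawns the targeter on BeginPlay and, while it is valid, sends it the cached look location and hit result every Tick through UpdateTargeterMessage.
; SetTargeterState destroys the targeter when true and respawns it at the cached destination when false.
; An unconnected branch for yawing toward that destination never runs.
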(event `self.ReceiveBeginPlay`
  (bind _returnvalue (`GameplayStatics.GetPlayerPawn` 0))
  (bind _returnvalue_2 (`|SpawnActorFromClass` (`self.TargeterClass`) (`KismetMathLibrary.MakeTransform` (0.0 0.0 0.0)) "Undefined" "MultiplyWithRoot" _returnvalue _returnvalue))
  (set `self.TargeterRef` _returnvalue_2))

(event `self.ReceiveTick`
  (params (DeltaSeconds :type "Float (single-precision)"))
  (bind _targeterref (`self.TargeterRef`)
    (:`then`
      (message `/Game/Blueprints/Interfaces/Targeter_BPI.UpdateTargeter` _targeterref (`self.CachedLookDestination`) (`self.CachedHitResult`)))
    (:`else`)))

(event `SetTargeterState`
  (params (TargeterState :type Boolean))
  (bind _returnvalue (`GameplayStatics.GetPlayerPawn` 0))
  (bind _output_get (set `self.Targeter State` TargeterState))
  (if _output_get
    (`self.K2_DestroyActor` (`self.TargeterRef`))
    (else
      (bind _returnvalue_2 (`|SpawnActorFromClass` (`self.TargeterClass`) (`KismetMathLibrary.Conv_VectorToTransform` (`self.CachedLookDestination`)) "Undefined" "MultiplyWithRoot" _returnvalue _returnvalue))
      (set `self.TargeterRef` _returnvalue_2))))

(fn `UserConstructionScript`)