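; BP_MagicMissle is a magic missile projectile actor that deals point damage to what it hits.
; The construction script feeds Speed into projectile movement and the Niagara trail's velocity, and passes Lifetime to the effect.
; A BeginPlay timer destroys it after Lifetime.
; On hit it spawns an arcane impact effect, applies physical-type damage along the owner's forward vector with the instigator controller as causer, then destroys itself.
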(event `self.ReceiveBeginPlay`
  (`KismetSystemLibrary.K2_SetTimerDelegate` (delegate `Destroy`) (`self.Lifetime`)))

(event `Destroy`
  (`self.K2_DestroyActor`))

(event `self.ReceiveHit`
  (params (MyComp :type "PrimitiveComponent Object Reference") (Other :type "Actor Object Reference") (OtherComp :type "PrimitiveComponent Object Reference") (bSelfMoved :type Boolean) (HitLocation :type "Vector Structure") (HitNormal :type "Vector Structure") (NormalImpulse :type "Vector Structure") (Hit :type "HitResult Structure (by ref)"))
  (bind (_bblockinghit _binitialoverlap _time _distance _location _impactpoint _normal _impactnormal _physmat _hitactor) (`GameplayStatics.BreakHitResult` Hit))
  (bind _returnvalue (`self.GetInstigatorController`))
  (`NiagaraFunctionLibrary.SpawnSystemAtLocation` "/Game/Assets/NS_ArcaneHit.NS_ArcaneHit" _location)
  (`GameplayStatics.ApplyPointDamage` _hitactor (`self.BaseDamage`) (`self.GetActorForwardVector` (`self.GetOwner`)) Hit _returnvalue _returnvalue "/Game/Blueprints/Enumerations/DT_PhysicalDamage.DT_PhysicalDamage_C")
  (`self.K2_DestroyActor`))

(fn `UserConstructionScript`
  (bind _niagara (`self.Niagara`))
  (set `ProjectileMovementComponent.InitialSpeed` (`self.Speed`) (`self.ProjectileMovement`))
  (`FXSystemComponent.SetVectorParameter` _niagara "Velocity" (`KismetMathLibrary.MakeVector` (`self.Speed`)))
  (`FXSystemComponent.SetFloatParameter` _niagara "Lifetime" (`self.Lifetime`)))