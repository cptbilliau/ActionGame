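; BP_BaseSkill is a base skill actor that scales its stats to the owner's skill level when it spawns.
; On BeginPlay it looks up its own class in the SkillLevelMap of the owner's BP_CombatComponent.
; That level linearly reduces cooldown and raises damage, healing and their attribute scaling values.
; It then sends the owner SlotFiredMessage with its attached slot and adjusted cooldown.
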(event `self.ReceiveBeginPlay`
  (`self.SetSkillLevel`)
  (message `/Game/Blueprints/Interfaces/Combat_BPI.SlotFired` (`self.GetOwner`) (`self.AttachedSlot`) (`self.BaseCooldown`)))

(fn `SetSkillLevel`
  (locals (ItemLevel :type Integer))
  (set `local.ItemLevel` (`BlueprintMapLibrary.Map_Find` (`CombatComponent.SkillLevelMap` (`self.GetComponentByClass` (`self.GetOwner`) "/Game/Blueprints/Components/BP_CombatComponent.BP_CombatComponent_C")) (`|ConvertAsset` (`GameplayStatics.GetObjectClass` self))))
  (`|ExecutionSequence`
    (:`then_0`
      (set `self.BaseCooldown` (- (`self.BaseCooldown`) (* (`local.ItemLevel`) (`self.CooldownReductionPerLevel`)))))
    (:`then_1`
      (set `self.MagicScaling` (+ (* (`local.ItemLevel`) (`self.MagicScalingPerLevel`)) (`self.MagicScaling`)))
      (set `self.MightScaling` (+ (* (`local.ItemLevel`) (`self.MightScalingPerLevel`)) (`self.MightScaling`)))
      (set `self.DevotionScaling` (+ (* (`local.ItemLevel`) (`self.DevotionScalingPerLevel`)) (`self.DevotionScaling`)))
      (set `self.BaseDamage` (+ (* (`local.ItemLevel`) (`self.BaseDamagePerLevel`)) (`self.BaseDamage`))))
    (:`then_2`
      (set `self.MagicHealScaling` (+ (* (`local.ItemLevel`) (`self.MagicHealScalingPerLevel`)) (`self.MagicHealScaling`)))
      (set `self.DevotionHealScaling` (+ (* (`local.ItemLevel`) (`self.DevotionHealScalingPerLevel`)) (`self.DevotionHealScaling`)))
      (set `self.BaseHealing` (+ (* (`local.ItemLevel`) (`self.BaseHealingPerLevel`)) (`self.BaseHealing`))))))

(fn `UserConstructionScript`)