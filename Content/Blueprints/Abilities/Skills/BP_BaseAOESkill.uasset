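; Base area-of-effect skill actor that repeatedly damages or heals actors in a radius until AOEDuration expires.
; Tick uses a Delay to pace sphere traces, then destroys the actor once the timer flags it.
; HitFunction applies point damage or healing-typed damage once per actor per pulse, team-checking ally modes but not Enemy mode.
; SetGroundTargeter traces vertically to find a flattish ground location.
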(event `self.ReceiveBeginPlay`
  (`parent.ReceiveBeginPlay`)
  (`KismetSystemLibrary.K2_SetTimerDelegate` (delegate `Destroy`) (`self.AOEDuration`)))

(event `Destroy`
  (set `self.ShouldDestroy?` true))

(event `self.ReceiveTick`
  (params (DeltaSeconds :type "Float (single-precision)"))
  (bind _returnvalue (`SceneComponent.K2_GetComponentLocation` (`self.DefaultSceneRoot`)))
  (`KismetSystemLibrary.Delay` (`self.DamageTickRate`))
  (if (`self.ShouldDestroy?`)
    (`self.K2_DestroyActor`)
    (else
      (bind _outhits (`KismetSystemLibrary.SphereTraceMultiForObjects` (`KismetMathLibrary.MakeVector` (.x _returnvalue) (.y _returnvalue) (+ (.z _returnvalue) 200.0)) _returnvalue (`self.AOERadius`) (`|MakeArray` "ObjectTypeQuery1" "ObjectTypeQuery3" "ObjectTypeQuery2" :!type "EObjectTypeQuery Enum") false (`|MakeArray` (`self.Instigator`) (`self.GetOwner`) :!type "Actor Object Reference") "None" true (struct :`R` 1.0 :`A` 1.0) (struct :`G` 1.0 :`A` 1.0) (`self.DamageTickRate`)))
      (`self.HitFunction` _outhits))))

(fn `HitFunction`
  (params (Array :type "Array of HitResult Structure"))
  (locals (L_HitActor :type "Actor Object Reference") (L_HitResult :type "HitResult Structure"))
  (bind _returnvalue (`self.GetComponentByClass` (`local.L_HitActor`) "/Game/Blueprints/Components/BP_CombatComponent.BP_CombatComponent_C"))
  (bind _returnvalue_2 (`self.GetComponentByClass` (`local.L_HitActor`) "/Game/Blueprints/Components/BP_CombatComponent.BP_CombatComponent_C"))
  (for _array_element Array
    (set `local.L_HitResult` _array_element)
    (bind _output_get (set `local.L_HitActor` (`.HitActor` (`GameplayStatics.BreakHitResult` _array_element))))
    (if (not (`KismetArrayLibrary.Array_Contains` (`self.Hit Actors Array`) _output_get))
      (switch `EAbilityTargetType` (`self.AbilityTargetType`)
        (:`E_Enemies`
          ;[1 1 1] Deal Damage
          (`GameplayStatics.ApplyPointDamage` (`local.L_HitActor`) (`self.GetAbilityDamage`) (`self.K2_GetActorLocation`) (`local.L_HitResult`) (`self.GetInstigatorController`) self (select `EAbilityDamageType` (`self.DamageType`) :`E_Physical` "/Game/Blueprints/Enumerations/DT_PhysicalDamage.DT_PhysicalDamage_C" :`E_Magical` "/Game/Blueprints/Enumerations/DT_MagicalDamage.DT_MagicalDamage_C" :!type "DamageType Class Reference") :!label _label)
          (`KismetArrayLibrary.Array_AddUnique` (`self.Hit Actors Array`) (`local.L_HitActor`) :!label _label_2))
        (:`E_Allies`
          (`/Engine/EditorBlueprintResources/StandardMacros.IsValid` _returnvalue_2
            (:`Is Valid`
              (if (== (`CombatComponent.Team` (`self.GetComponentByClass` (`self.Instigator`) "/Game/Blueprints/Components/BP_CombatComponent.BP_CombatComponent_C")) (`CombatComponent.Team` _returnvalue_2))
                ;[1 1 1] Deal Healing
                (`GameplayStatics.ApplyPointDamage` (`local.L_HitActor`) (`self.GetAbilityHealing`) (`self.K2_GetActorLocation`) (`local.L_HitResult`) (`self.GetInstigatorController`) self "/Game/Blueprints/Enumerations/DT_HealingDamage.DT_HealingDamage_C" :!label _label_3)
                (goto _label_2)))))
        (:`E_AlliesAndEnemies`
          (`/Engine/EditorBlueprintResources/StandardMacros.IsValid` _returnvalue
            (:`Is Valid`
              (if (== (`CombatComponent.Team` (`self.GetComponentByClass` (`self.Instigator`) "/Game/Blueprints/Components/BP_CombatComponent.BP_CombatComponent_C")) (`CombatComponent.Team` _returnvalue))
                (goto _label_3)
                (else
                  (goto _label)))))))))
  (`KismetArrayLibrary.Array_Clear` (`self.Hit Actors Array`)))

(fn `SetGroundTargeter`
  (params (HitLocation :type "Vector Structure") (HitResult :type "HitResult Structure"))
  (returns (NewParam :type "Vector Structure"))
  (locals (NewLocalVar :type Boolean :default true) (NewLocalVar_0 :type "Vector Structure" :default (0.0 0.0 0.0)) (L_GroundHits :type "Array of HitResult Structure"))
  (bind _l_groundhits (`local.L_GroundHits`))
  (bind (_bblockinghit _binitialoverlap _time _distance _location _impactpoint _normal _impactnormal) (`GameplayStatics.BreakHitResult` (`|GetArrayItem` _l_groundhits)))
  (bind (_returnvalue_roll _returnvalue_pitch) (`KismetMathLibrary.BreakRotator` (`KismetMathLibrary.Conv_VectorToRotator` _impactnormal)))
  (bind _outhits (`KismetSystemLibrary.SphereTraceMultiForObjects` :`Start` (`KismetMathLibrary.MakeVector` (.x HitLocation) (.y HitLocation) (+ (.z HitLocation) 20.0)) :`End` (`KismetMathLibrary.MakeVector` (.x HitLocation) (.y HitLocation) (- (.z HitLocation) 500.0)) :`Radius` 3.0 :`ObjectTypes` (`|MakeArray` "ObjectTypeQuery1" "ObjectTypeQuery2" :!type "EObjectTypeQuery Enum") :`DrawDebugType` "ForOneFrame"))
  (for _array_element _outhits
    (`KismetArrayLibrary.Array_AddUnique` _l_groundhits _array_element)
    (if (`KismetMathLibrary.InRange_FloatFloat` _returnvalue_pitch 30.0 90.0)
      (return _location)
      (else
        (`KismetArrayLibrary.Array_RemoveItem` _l_groundhits _array_element))))
  (`KismetArrayLibrary.Array_Clear` (`local.L_GroundHits`)))

(fn `UserConstructionScript`)