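; BP_AxeThrow is a thrown-axe skill actor that spins in flight and sticks into the world on impact.
; Tick rotates its Niagara component in pitch by a fixed step per frame, not scaled by delta time.
; On hitting a WorldStatic or WorldDynamic component, it prints that component's name, spawns NS_Axe_Stuck at the impact point with the axe's current rotation and scale, then destroys itself.
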(event `self.ReceiveTick`
  (params (DeltaSeconds :type "Float (single-precision)"))
  (`parent.ReceiveTick` DeltaSeconds)
  (`SceneComponent.K2_AddLocalRotation` (`self.Niagara`) (`KismetMathLibrary.MakeRotator` 0.0 -10.0) false false))

(event `self.ReceiveHit`
  (params (MyComp :type "PrimitiveComponent Object Reference") (Other :type "Actor Object Reference") (OtherComp :type "PrimitiveComponent Object Reference") (bSelfMoved :type Boolean) (HitLocation :type "Vector Structure") (HitNormal :type "Vector Structure") (NormalImpulse :type "Vector Structure") (Hit :type "HitResult Structure (by ref)"))
  (bind (_bblockinghit _binitialoverlap _time _distance _location _impactpoint _normal _impactnormal _physmat _hitactor _hitcomponent) (`GameplayStatics.BreakHitResult` Hit))
  (bind _returnvalue (`PrimitiveComponent.GetCollisionObjectType` _hitcomponent))
  (set `self.AxeScale` (`SceneComponent.K2_GetComponentScale` (`self.Niagara`)))
  (set `self.NewVar` (`SceneComponent.K2_GetComponentRotation` (`self.Niagara`)))
  (if (or (`|EnumEquality` _returnvalue "ECC_WorldStatic") (`|EnumEquality` _returnvalue "ECC_WorldDynamic"))
    (`KismetSystemLibrary.PrintString` (`KismetSystemLibrary.GetDisplayName` _hitcomponent))
    (`NiagaraFunctionLibrary.SpawnSystemAtLocation` "/Game/VFX/RPGEffects/ParticlesNiagara/Warrior/ThrowingAxe/NS_Axe_Stuck.NS_Axe_Stuck" _location (`self.NewVar`) (`self.AxeScale`))
    (`self.K2_DestroyActor`)))

(fn `UserConstructionScript`
  (`parent.UserConstructionScript`))