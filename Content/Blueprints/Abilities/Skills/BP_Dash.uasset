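; BP_Dash is a dash skill that launches its owning character along its current velocity.
; On BeginPlay it casts its owner to Character, caches the reference and prints debug strings for the result.
; A custom event calls LaunchCharacter with triple the owner's velocity, overriding horizontal velocity only.
; BaseCooldown is unused, so no cooldown is applied, and nothing in this graph calls the dash event.
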(event `self.ReceiveBeginPlay`
  (`KismetSystemLibrary.PrintString` "Hello")
  (bind _ascharacter (cast `Character` (`self.GetOwner`))
    (:`then`
      (set `self.As Character` _ascharacter)
      (`KismetSystemLibrary.PrintString` "yes"))
    (:`CastFailed`
      (`KismetSystemLibrary.PrintString` "fail"))))

(event `CustomEvent`
  (`Character.LaunchCharacter` (`self.As Character`) (* (`self.GetVelocity` (`self.GetOwner`)) 3.0) true false))

(fn `UserConstructionScript`)