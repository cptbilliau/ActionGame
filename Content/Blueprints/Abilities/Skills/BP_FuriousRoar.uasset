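; Furious Roar skill actor that knocks hit characters away from its owner and up into the air as soon as it spawns.
; BeginPlay runs the parent logic, then loops over HitActorsArray, which is not filled in this graph.
; Each Character is launched along the look-at direction from the owner plus an upward bias, scaled per axis and overriding its current velocity.
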(event `self.ReceiveBeginPlay`
  (`parent.ReceiveBeginPlay`)
  (for _array_element (`self.Hit Actors Array`)
    (bind _ascharacter (cast `Character` _array_element))
    (`Character.LaunchCharacter` _ascharacter (* (+ (`KismetMathLibrary.Conv_RotatorToVector` (`KismetMathLibrary.FindLookAtRotation` (`self.K2_GetActorLocation` (`self.GetOwner`)) (`self.K2_GetActorLocation` _array_element))) (0.0 0.0 1.0)) (200.0 200.0 400.0)) true true)))

(fn `UserConstructionScript`
  (`parent.UserConstructionScript`))