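; BP_Dash is a dash movement ability actor that launches its owning Character along its current velocity.
; On BeginPlay it prints a debug string, casts its owner to Character and chains a server-named event into a client-named one.
; The client event calls LaunchCharacter with a multiple of the owner's velocity, overriding horizontal velocity and adding to vertical.
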(event `self.ReceiveBeginPlay`
  (`KismetSystemLibrary.PrintString` "Hello")
  (bind _ascharacter (cast `Character` (`self.GetOwner`)))
  (set `self.As Character` _ascharacter)
  (`self.Server_LaunchCharacter`))

(event `Server_LaunchCharacter`
  (`self.Client_LaunchCharacter`))

(event `Client_LaunchCharacter`
  (`Character.LaunchCharacter` (`self.As Character`) (* (`self.GetVelocity` (`self.GetOwner`)) 4.0) true false))

(fn `UserConstructionScript`)