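; BP_Blink is a blink movement skill actor that relocates its owner to the spot where the actor stands.
; On BeginPlay it spawns an arcane hit Niagara effect slightly above itself, then waits briefly before triggering the teleport.
; A server event calls a client event, which sets the owner's location to a raised point above the actor, without sweep.
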(event `self.ReceiveBeginPlay`
  (`NiagaraFunctionLibrary.SpawnSystemAtLocation` "/Game/Assets/NS_ArcaneHit.NS_ArcaneHit" (+ (`self.K2_GetActorLocation`) (0.0 0.0 90.0)))
  (`KismetSystemLibrary.Delay` 0.5)
  (`self.Server_TPplayer`))

(event `Server_TPplayer`
  (`self.Client_TPPlayer`))

(event `Client_TPPlayer`
  (`self.K2_SetActorLocation` (`self.GetOwner`) (+ (`self.K2_GetActorLocation`) (0.0 0.0 180.0)) false false))

(fn `UserConstructionScript`)