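; Fireball skill projectile that explodes on hit or overlap, or expires after its lifetime.
; On BeginPlay it scales cooldown, damage and healing by the owner's skill level, then reports cooldown to the owner's slot.
; Impact runs a sphere trace into HitFunction, which affects each actor once through point damage.
; Enemy mode damages without team checks; both ally modes heal teammates via a healing damage type and damage other combatants.
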(event `self.ReceiveBeginPlay`
  (`self.SetSkillLevel`)
  (message `/Game/Blueprints/Interfaces/Combat_BPI.SlotFired` (`self.GetOwner`) (`self.AttachedSlot`) (`self.BaseCooldown`))
  (`KismetSystemLibrary.K2_SetTimerDelegate` (delegate `Destroy`) (`self.Lifetime`)))

(event `Destroy`
  (`self.K2_DestroyActor`))

(event `self.Sphere.OnComponentHit`
  (params (HitComponent :type "PrimitiveComponent Object Reference") (OtherActor :type "Actor Object Reference") (OtherComp :type "PrimitiveComponent Object Reference") (NormalImpulse :type "Vector Structure") (Hit :type "HitResult Structure (by ref)"))
  (bind (_bblockinghit _binitialoverlap _time _distance _location _impactpoint _normal _impactnormal _physmat _hitactor) (`GameplayStatics.BreakHitResult` Hit))
  (if (and (!= _hitactor (`self.GetOwner`)) (!= _hitactor self))
    (`GameplayStatics.SpawnEmitterAtLocation` "/Game/VFX/FXVarietyPack/Particles/P_ky_explosion.P_ky_explosion" _location (struct) (0.6 0.6 0.6))
    (bind _outhits (`KismetSystemLibrary.SphereTraceMultiForObjects` _location _location 130.0 (`|MakeArray` "ObjectTypeQuery1" "ObjectTypeQuery3" "ObjectTypeQuery2" :!type "EObjectTypeQuery Enum") false (`|MakeArray` (`self.Instigator`) (`self.GetOwner`) :!type "Actor Object Reference")))
    (`self.HitFunction` _outhits)
    (`KismetArrayLibrary.Array_Clear` (`self.Hit Actors Array`))
    (`self.K2_DestroyActor`)))

(event `self.Sphere.OnComponentBeginOverlap`
  (params (OverlappedComponent :type "PrimitiveComponent Object Reference") (OtherActor :type "Actor Object Reference") (OtherComp :type "PrimitiveComponent Object Reference") (OtherBodyIndex :type Integer) (bFromSweep :type Boolean) (SweepResult :type "HitResult Structure (by ref)"))
  (bind (_bblockinghit _binitialoverlap _time _distance _location _impactpoint _normal _impactnormal _physmat _hitactor) (`GameplayStatics.BreakHitResult` SweepResult))
  (if (and (!= _hitactor (`self.GetOwner`)) (!= _hitactor self))
    (`GameplayStatics.SpawnEmitterAtLocation` "/Game/VFX/FXVarietyPack/Particles/P_ky_explosion.P_ky_explosion" _location (struct) (0.6 0.6 0.6))
    (bind _outhits (`KismetSystemLibrary.SphereTraceMultiForObjects` _location _location 130.0 (`|MakeArray` "ObjectTypeQuery1" "ObjectTypeQuery3" "ObjectTypeQuery2" :!type "EObjectTypeQuery Enum") false (`|MakeArray` (`self.Instigator`) (`self.GetOwner`) :!type "Actor Object Reference")))
    (`self.HitFunction` _outhits)
    (`KismetArrayLibrary.Array_Clear` (`self.Hit Actors Array`))
    (`self.K2_DestroyActor`)))

(fn `HitFunction`
  (params (Array :type "Array of HitResult Structure"))
  (locals (L_HitActor :type "Actor Object Reference") (L_HitResult :type "HitResult Structure"))
  (bind _returnvalue (`self.GetComponentByClass` (`local.L_HitActor`) "/Game/Blueprints/Components/BP_CombatComponent.BP_CombatComponent_C"))
  (bind _returnvalue_2 (`self.GetComponentByClass` (`local.L_HitActor`) "/Game/Blueprints/Components/BP_CombatComponent.BP_CombatComponent_C"))
  (for _array_element Array
    (set `local.L_HitResult` _array_element)
    (bind _output_get (set `local.L_HitActor` (`.HitActor` (`GameplayStatics.BreakHitResult` _array_element))))
    (if (not (`KismetArrayLibrary.Array_Contains` (`self.Hit Actors Array`) _output_get))
      (switch `EAbilityTargetType` (`self.AbilityTargetType`)
        (:`E_Enemies`
          ;[1 1 1] Deal Damage
          (`GameplayStatics.ApplyPointDamage` (`local.L_HitActor`) (`self.GetAbilityDamage`) (`self.K2_GetActorLocation`) (`local.L_HitResult`) (`self.GetInstigatorController`) self (select `EAbilityDamageType` (`self.DamageType`) :`E_Physical` "/Game/Blueprints/Enumerations/DT_PhysicalDamage.DT_PhysicalDamage_C" :`E_Magical` "/Game/Blueprints/Enumerations/DT_MagicalDamage.DT_MagicalDamage_C" :!type "DamageType Class Reference") :!label _label))
        (:`E_Allies`
          (`/Engine/EditorBlueprintResources/StandardMacros.IsValid` _returnvalue_2
            (:`Is Valid`
              (if (== (`CombatComponent.Team` (`self.GetComponentByClass` (`self.Instigator`) "/Game/Blueprints/Components/BP_CombatComponent.BP_CombatComponent_C")) (`CombatComponent.Team` _returnvalue_2))
                ;[1 1 1] Deal Healing
                (`GameplayStatics.ApplyPointDamage` (`local.L_HitActor`) (`self.GetAbilityHealing`) (`self.K2_GetActorLocation`) (`local.L_HitResult`) (`self.GetInstigatorController`) self "/Game/Blueprints/Enumerations/DT_HealingDamage.DT_HealingDamage_C" :!label _label_2)
                (else
                  (goto _label))))))
        (:`E_AlliesAndEnemies`
          (`/Engine/EditorBlueprintResources/StandardMacros.IsValid` _returnvalue
            (:`Is Valid`
              (if (== (`CombatComponent.Team` (`self.GetComponentByClass` (`self.Instigator`) "/Game/Blueprints/Components/BP_CombatComponent.BP_CombatComponent_C")) (`CombatComponent.Team` _returnvalue))
                (goto _label_2)
                (else
                  (goto _label)))))))
      (`KismetArrayLibrary.Array_AddUnique` (`self.Hit Actors Array`) (`local.L_HitActor`)))))

(fn `SetSkillLevel`
  (locals (ItemLevel :type Integer))
  (set `local.ItemLevel` (`BlueprintMapLibrary.Map_Find` (`CombatComponent.SkillLevelMap` (`self.GetComponentByClass` (`self.GetOwner`) "/Game/Blueprints/Components/BP_CombatComponent.BP_CombatComponent_C")) (`|ConvertAsset` (`GameplayStatics.GetObjectClass` self))))
  (`|ExecutionSequence`
    (:`then_0`
      (set `self.BaseCooldown` (- (`self.BaseCooldown`) (* (`local.ItemLevel`) (`self.CooldownReductionPerLevel`)))))
    (:`then_1`
      (set `self.MagicScaling` (+ (* (`local.ItemLevel`) (`self.MagicScalingPerLevel`)) (`self.MagicScaling`)))
      (set `self.MightScaling` (+ (* (`local.ItemLevel`) (`self.MightScalingPerLevel`)) (`self.MightScaling`)))
      (set `self.DevotionScaling` (+ (* (`local.ItemLevel`) (`self.DevotionScalingPerLevel`)) (`self.DevotionScaling`)))
      (set `self.BaseDamage` (+ (* (`local.ItemLevel`) (`self.BaseDamagePerLevel`)) (`self.BaseDamage`))))
    (:`then_2`
      (set `self.MagicHealScaling` (+ (* (`local.ItemLevel`) (`self.MagicHealScalingPerLevel`)) (`self.MagicHealScaling`)))
      (set `self.DevotionHealScaling` (+ (* (`local.ItemLevel`) (`self.DevotionHealScalingPerLevel`)) (`self.DevotionHealScaling`)))
      (set `self.BaseHealing` (+ (* (`local.ItemLevel`) (`self.BaseHealingPerLevel`)) (`self.BaseHealing`))))))

(fn `UserConstructionScript`
  (set `ProjectileMovementComponent.InitialSpeed` (`self.Speed`) (`self.ProjectileMovement`))
  (`FXSystemComponent.SetFloatParameter` (`self.Niagara`) "Lifetime" (`self.Lifetime`)))