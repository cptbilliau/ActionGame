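; Base projectile for ability skills that scales with skill level, reports its cooldown to the owner and expires after a lifetime.
; Construction feeds speed and lifetime into the movement component and Niagara effect.
; Sphere overlap with anything but the owner applies typed point damage, spawns a hit effect and destroys the projectile.
; A separate HitFunction, not called here, applies team-based damage or healing-as-damage, recording actors hit.
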(event `self.ReceiveBeginPlay`
  (`self.SetSkillLevel`)
  (message `/Game/Blueprints/Interfaces/Combat_BPI.SlotFired` (`self.GetOwner`) (`self.AttachedSlot`) (`self.BaseCooldown`))
  (`KismetSystemLibrary.K2_SetTimerDelegate` (delegate `Destroy`) (`self.Lifetime`)))

(event `Destroy`
  (`self.K2_DestroyActor`))

(event `self.ReceiveTick`
  (params (DeltaSeconds :type "Float (single-precision)")))

(event `self.Sphere.OnComponentBeginOverlap`
  (params (OverlappedComponent :type "PrimitiveComponent Object Reference") (OtherActor :type "Actor Object Reference") (OtherComp :type "PrimitiveComponent Object Reference") (OtherBodyIndex :type Integer) (bFromSweep :type Boolean) (SweepResult :type "HitResult Structure (by ref)"))
  (bind (_bblockinghit _binitialoverlap _time _distance _location _impactpoint _normal _impactnormal _physmat _hitactor) (`GameplayStatics.BreakHitResult` SweepResult))
  (if (and (!= _hitactor (`self.GetOwner`)) (!= _hitactor self))
    (`KismetSystemLibrary.PrintString` "Hit")
    (`GameplayStatics.ApplyPointDamage` _hitactor (`self.GetAbilityDamage`) (`self.GetActorForwardVector` (`self.GetOwner`)) SweepResult (`self.GetInstigatorController`) self (select `EAbilityDamageType` (`self.DamageType`) :`E_Physical` "/Game/Blueprints/Enumerations/DT_PhysicalDamage.DT_PhysicalDamage_C" :`E_Magical` "/Game/Blueprints/Enumerations/DT_MagicalDamage.DT_MagicalDamage_C" :!type "DamageType Class Reference"))
    (`NiagaraFunctionLibrary.SpawnSystemAtLocation` (`self.HitEffect`))
    (`self.K2_DestroyActor`)))

(fn `HitFunction`
  (params (Array :type "Array of HitResult Structure"))
  (locals (L_HitActor :type "Actor Object Reference") (L_HitResult :type "HitResult Structure"))
  (bind _returnvalue (`self.GetComponentByClass` (`local.L_HitActor`) "/Game/Blueprints/Components/BP_CombatComponent.BP_CombatComponent_C"))
  (bind _returnvalue_2 (`self.GetComponentByClass` (`local.L_HitActor`) "/Game/Blueprints/Components/BP_CombatComponent.BP_CombatComponent_C"))
  (bind _returnvalue_3 (`self.GetComponentByClass` (`local.L_HitActor`) "/Game/Blueprints/Components/BP_CombatComponent.BP_CombatComponent_C"))
  (for _array_element Array
    (set `local.L_HitResult` _array_element)
    (bind _output_get (set `local.L_HitActor` (`.HitActor` (`GameplayStatics.BreakHitResult` _array_element))))
    (if (not (`KismetArrayLibrary.Array_Contains` (`self.Hit Actors Array`) _output_get))
      (switch `EAbilityTargetType` (`self.AbilityTargetType`)
        (:`E_Enemies`
          (`/Engine/EditorBlueprintResources/StandardMacros.IsValid` _returnvalue_2
            (:`Is Valid`
              ;[1 1 1] Deal Damage
              (if (!= (`CombatComponent.Team` (`self.GetComponentByClass` (`self.Instigator`) "/Game/Blueprints/Components/BP_CombatComponent.BP_CombatComponent_C")) (`CombatComponent.Team` _returnvalue_2)) :!label _label
                (`GameplayStatics.ApplyPointDamage` (`local.L_HitActor`) (`self.GetAbilityDamage`) (`self.K2_GetActorLocation`) (`local.L_HitResult`) (`self.GetInstigatorController`) self (select `EAbilityDamageType` (`self.DamageType`) :`E_Physical` "/Game/Blueprints/Enumerations/DT_PhysicalDamage.DT_PhysicalDamage_C" :`E_Magical` "/Game/Blueprints/Enumerations/DT_MagicalDamage.DT_MagicalDamage_C" :!type "DamageType Class Reference"))
                (`KismetArrayLibrary.Array_AddUnique` (`self.Hit Actors Array`) (`local.L_HitActor`) :!label _label_2)))))
        (:`E_Allies`
          (`/Engine/EditorBlueprintResources/StandardMacros.IsValid` _returnvalue_3
            (:`Is Valid`
              (if (== (`CombatComponent.Team` (`self.GetComponentByClass` (`self.Instigator`) "/Game/Blueprints/Components/BP_CombatComponent.BP_CombatComponent_C")) (`CombatComponent.Team` _returnvalue_3))
                ;[1 1 1] Deal Healing
                (`GameplayStatics.ApplyPointDamage` (`local.L_HitActor`) (`self.GetAbilityHealing`) (`self.K2_GetActorLocation`) (`local.L_HitResult`) (`self.GetInstigatorController`) self "/Game/Blueprints/Enumerations/DT_HealingDamage.DT_HealingDamage_C" :!label _label_3)
                (goto _label_2)
                (else
                  (goto _label))))))
        (:`E_AlliesAndEnemies`
          (`/Engine/EditorBlueprintResources/StandardMacros.IsValid` _returnvalue
            (:`Is Valid`
              (if (== (`CombatComponent.Team` (`self.GetComponentByClass` (`self.Instigator`) "/Game/Blueprints/Components/BP_CombatComponent.BP_CombatComponent_C")) (`CombatComponent.Team` _returnvalue))
                (goto _label_3)
                (else
                  (goto _label))))))))))

(fn `SetSkillLevel`
  (`|ExecutionSequence`
    (:`then_0`
      (set `self.BaseCooldown` (- (`self.BaseCooldown`) (* (`self.SkillLevel`) (`self.CooldownReductionPerLevel`)))))
    (:`then_1`
      (set `self.MagicScaling` (+ (* (`self.SkillLevel`) (`self.MagicScalingPerLevel`)) (`self.MagicScaling`)))
      (set `self.MightScaling` (+ (* (`self.SkillLevel`) (`self.MightScalingPerLevel`)) (`self.MightScaling`)))
      (set `self.DevotionScaling` (+ (* (`self.SkillLevel`) (`self.DevotionScalingPerLevel`)) (`self.DevotionScaling`)))
      (set `self.BaseDamage` (+ (* (`self.SkillLevel`) (`self.BaseDamagePerLevel`)) (`self.BaseDamage`))))
    (:`then_2`
      (set `self.MagicHealScaling` (+ (* (`self.SkillLevel`) (`self.MagicHealScalingPerLevel`)) (`self.MagicHealScaling`)))
      (set `self.DevotionHealScaling` (+ (* (`self.SkillLevel`) (`self.DevotionHealScalingPerLevel`)) (`self.DevotionHealScaling`)))
      (set `self.BaseHealing` (+ (* (`self.SkillLevel`) (`self.BaseHealingPerLevel`)) (`self.BaseHealing`))))))

(fn `UserConstructionScript`
  (set `ProjectileMovementComponent.InitialSpeed` (`self.Speed`) (`self.ProjectileMovement`))
  (`FXSystemComponent.SetFloatParameter` (`self.Niagara`) "Lifetime" (`self.Lifetime`)))