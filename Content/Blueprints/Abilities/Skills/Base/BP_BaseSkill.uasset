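; Base actor for skills, holding cooldown, area, damage and healing stats that scale with skill level.
; The construction script calls SetSkillLevel, which lowers cooldown and raises radius, base damage, base healing and attribute scalings linearly per level.
; Range is multiplied into the same pattern with a zero increment, so it stays constant.
; On BeginPlay it reports its attached slot and adjusted cooldown to its owner through SlotFiredMessage.
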(event `self.ReceiveBeginPlay`
  (message `/Game/Blueprints/Interfaces/Combat_BPI.SlotFired` (`self.GetOwner`) (`self.AttachedSlot`) (`self.BaseCooldown`)))

(fn `SetSkillLevel`
  (`|ExecutionSequence`
    (:`then_0`
      (set `self.BaseCooldown` (- (`self.BaseCooldown`) (* (`self.SkillLevel`) (`self.CooldownReductionPerLevel`))))
      (set `self.Radius` (+ (`self.Radius`) (* (`self.SkillLevel`) (`self.RadiusPerLevel`))))
      (set `self.Range` (+ (`self.Range`) (* (`self.SkillLevel`) 0.0))))
    (:`then_1`
      (set `self.MagicScaling` (+ (* (`self.SkillLevel`) (`self.MagicScalingPerLevel`)) (`self.MagicScaling`)))
      (set `self.MightScaling` (+ (* (`self.SkillLevel`) (`self.MightScalingPerLevel`)) (`self.MightScaling`)))
      (set `self.DevotionScaling` (+ (* (`self.SkillLevel`) (`self.DevotionScalingPerLevel`)) (`self.DevotionScaling`)))
      (set `self.BaseDamage` (+ (* (`self.SkillLevel`) (`self.BaseDamagePerLevel`)) (`self.BaseDamage`))))
    (:`then_2`
      (set `self.MagicHealScaling` (+ (* (`self.SkillLevel`) (`self.MagicHealScalingPerLevel`)) (`self.MagicHealScaling`)))
      (set `self.DevotionHealScaling` (+ (* (`self.SkillLevel`) (`self.DevotionHealScalingPerLevel`)) (`self.DevotionHealScaling`)))
      (set `self.BaseHealing` (+ (* (`self.SkillLevel`) (`self.BaseHealingPerLevel`)) (`self.BaseHealing`))))))

(fn `UserConstructionScript`
  (`self.SetSkillLevel`))