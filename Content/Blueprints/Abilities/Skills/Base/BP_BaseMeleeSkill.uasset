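; Base melee skill actor that strikes everything in an arc in front of it on spawn.
; BeginPlay rotates back by half the Radius angle, then steps by RotationAmount, firing a multi-object line trace of Range length at each step.
; HitFunction compares BP_CombatComponent teams by AbilityTargetType, applying damage or healing through ApplyPointDamage once per actor.
; The Allies mode also damages opposing teams, exactly like Allies & Enemies.
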(event `CalculateRotationSteps`
  (set `self.LineCastAmount` (`KismetMathLibrary.FTrunc` (/ (`self.Radius`) (`self.RotationAmount`))))
  (`self.K2_AddActorWorldRotation` (`KismetMathLibrary.MakeRotator` 0.0 0.0 (* (/ (`self.Radius`) 2.0) -1.0))))

(event `self.ReceiveBeginPlay`
  (bind _returnvalue (`self.K2_GetActorLocation`))
  (`KismetArrayLibrary.Array_Clear` (`self.Hit Actors Array`))
  (`parent.ReceiveBeginPlay`)
  (`|ExecutionSequence`
    (:`then_0`
      (`self.CalculateRotationSteps`))
    (:`then_1`
      (for _ (range (+ (`self.LineCastAmount`) 1)) :!label _label
        (bind _outhits (`KismetSystemLibrary.LineTraceMultiForObjects` _returnvalue (+ _returnvalue (* (`KismetMathLibrary.GetForwardVector` (`self.K2_GetActorRotation`)) (`self.Range`))) (`|MakeArray` "ObjectTypeQuery1" "ObjectTypeQuery3" "ObjectTypeQuery2" :!type "EObjectTypeQuery Enum") false (select `EAbilityTargetType` (`self.AbilityTargetType`) :`E_Enemies` (`|MakeArray` (`self.Instigator`) (`self.GetOwner`) :!type "Actor Object Reference")) (`self.Draw Debug Type`) false (struct :`R` 1.0 :`A` 1.0) (struct :`G` 1.0 :`A` 1.0) 0.5))
        (`self.K2_AddActorWorldRotation` (`KismetMathLibrary.MakeRotator` 0.0 0.0 (`self.RotationAmount`)))
        (bind _output_get (set `self.HitArray` _outhits))
        (`self.HitFunction` _output_get)))))

(event `BreakLoop`
  (goto _label :!via `Break`))

(fn `HitFunction`
  (params (Array :type "Array of HitResult Structure"))
  (locals (L_HitActor :type "Actor Object Reference") (L_HitResult :type "HitResult Structure"))
  (bind _healingout (`self.GetAbilityHealing`))
  (bind _returnvalue (`self.GetComponentByClass` (`local.L_HitActor`) "/Game/Blueprints/Components/BP_CombatComponent.BP_CombatComponent_C"))
  (bind _returnvalue_2 (`self.GetComponentByClass` (`local.L_HitActor`) "/Game/Blueprints/Components/BP_CombatComponent.BP_CombatComponent_C"))
  (bind _returnvalue_3 (`self.GetComponentByClass` (`local.L_HitActor`) "/Game/Blueprints/Components/BP_CombatComponent.BP_CombatComponent_C"))
  (for _array_element Array
    (set `local.L_HitResult` _array_element)
    (bind _output_get (set `local.L_HitActor` (`.HitActor` (`GameplayStatics.BreakHitResult` _array_element))))
    (if (not (`KismetArrayLibrary.Array_Contains` (`self.Hit Actors Array`) _output_get))
      (switch `EAbilityTargetType` (`self.AbilityTargetType`)
        (:`E_Enemies`
          (`/Engine/EditorBlueprintResources/StandardMacros.IsValid` _returnvalue_2
            (:`Is Valid`
              (if (!= (`CombatComponent.Team` (`self.GetComponentByClass` (`self.Instigator`) "/Game/Blueprints/Components/BP_CombatComponent.BP_CombatComponent_C")) (`CombatComponent.Team` _returnvalue_2)) :!label _label
                ;[1 1 1] Deal Damage
                (`GameplayStatics.ApplyPointDamage` (`local.L_HitActor`) (`self.GetAbilityDamage`) (`self.K2_GetActorLocation`) (`local.L_HitResult`) (`self.GetInstigatorController`) self (select `EAbilityDamageType` (`self.DamageType`) :`E_Physical` "/Game/Blueprints/Enumerations/DT_PhysicalDamage.DT_PhysicalDamage_C" :`E_Magical` "/Game/Blueprints/Enumerations/DT_MagicalDamage.DT_MagicalDamage_C" :!type "DamageType Class Reference"))
                (`KismetArrayLibrary.Array_AddUnique` (`self.Hit Actors Array`) (`local.L_HitActor`) :!label _label_2)))))
        (:`E_Allies`
          (`/Engine/EditorBlueprintResources/StandardMacros.IsValid` _returnvalue_3
            (:`Is Valid`
              (if (== (`CombatComponent.Team` (`self.GetComponentByClass` (`self.Instigator`) "/Game/Blueprints/Components/BP_CombatComponent.BP_CombatComponent_C")) (`CombatComponent.Team` _returnvalue_3))
                ;[1 1 1] Deal Healing
                (`KismetSystemLibrary.PrintString` (`KismetStringLibrary.Conv_DoubleToString` _healingout) :!label _label_3)
                (`GameplayStatics.ApplyPointDamage` (`local.L_HitActor`) _healingout (`self.K2_GetActorLocation`) (`local.L_HitResult`) (`self.GetInstigatorController`) self "/Game/Blueprints/Enumerations/DT_HealingDamage.DT_HealingDamage_C")
                (goto _label_2)
                (else
                  (goto _label))))))
        (:`E_AlliesAndEnemies`
          (`/Engine/EditorBlueprintResources/StandardMacros.IsValid` _returnvalue
            (:`Is Valid`
              (if (== (`CombatComponent.Team` (`self.GetComponentByClass` (`self.Instigator`) "/Game/Blueprints/Components/BP_CombatComponent.BP_CombatComponent_C")) (`CombatComponent.Team` _returnvalue))
                (goto _label_3)
                (else
                  (goto _label))))))))))

(fn `UserConstructionScript`)