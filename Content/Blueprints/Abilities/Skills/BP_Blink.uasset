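; BP_Blink is a movement-slot ability actor that attempts a teleport to just above its own location.
; On BeginPlay it prints a debug string, reports the fired slot and cooldown to its owner, and spawns an arcane-hit Niagara effect.
; After a short delay it teleports, without sweep, the owner's instigator controller rather than the owner itself.
; An unconnected node that would move the owner directly never runs.
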(event `self.ReceiveBeginPlay`
  (bind _returnvalue (+ (`self.K2_GetActorLocation`) (0.0 0.0 90.0)))
  (`KismetSystemLibrary.PrintString` "Hello")
  (message `/Game/Blueprints/Interfaces/Combat_BPI.SlotFired` (`self.GetOwner`) "E_MovementSlot" (`self.BaseCooldown`))
  (`NiagaraFunctionLibrary.SpawnSystemAtLocation` "/Game/Assets/NS_ArcaneHit.NS_ArcaneHit" _returnvalue)
  (`KismetSystemLibrary.Delay` 0.2)
  (`self.K2_SetActorLocation` (`self.GetInstigatorController` (`self.GetOwner`)) _returnvalue false true))

(fn `UserConstructionScript`)