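; Hail of Arrows skill actor that drives the Niagara effect for an area ability, extending parent class behavior.
; On BeginPlay it passes its Radius to the Niagara Radius parameter.
; Tick runs through a Delay of DamageTickRate, restarting the effect at that interval unless ShouldDestroy is set.
; This graph applies no damage itself.
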(event `self.ReceiveBeginPlay`
  (`parent.ReceiveBeginPlay`)
  (`NiagaraComponent.SetVariableFloat` (`self.Niagara`) "Radius" (`self.Radius`)))

(event `self.ReceiveTick`
  (params (DeltaSeconds :type "Float (single-precision)"))
  (`parent.ReceiveTick` DeltaSeconds)
  (`KismetSystemLibrary.Delay` (`self.DamageTickRate`))
  (if (not (`self.ShouldDestroy?`))
    (`NiagaraComponent.ResetSystem` (`self.Niagara`))))

(fn `UserConstructionScript`
  (`parent.UserConstructionScript`))