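; Base area-of-effect skill actor that deals repeated damage around its location for a set duration.
; Tick uses a Delay as the damage interval, sphere-tracing from above and applying physical or magical point damage to hits, ignoring instigator and owner.
; A BeginPlay timer sets a flag, so destruction waits for the next damage interval.
; SetGroundTargeter traces down from a given location to return a flat-enough ground point for targeting.
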(event `self.ReceiveBeginPlay`
  (`KismetSystemLibrary.K2_SetTimerDelegate` (delegate `Destroy`) (`self.AOEDuration`)))

(event `Destroy`
  (set `self.ShouldDestroy?` true))

(event `self.ReceiveTick`
  (params (DeltaSeconds :type "Float (single-precision)"))
  (bind _returnvalue (`self.GetInstigatorController`))
  (bind _returnvalue_2 (`SceneComponent.K2_GetComponentLocation` (`self.DefaultSceneRoot`)))
  (`KismetSystemLibrary.Delay` (`self.DamageTickRate`))
  (if (`self.ShouldDestroy?`)
    (`self.K2_DestroyActor`)
    (else
      (bind _outhits (`KismetSystemLibrary.SphereTraceMultiForObjects` (`KismetMathLibrary.MakeVector` (.x _returnvalue_2) (.y _returnvalue_2) (+ (.z _returnvalue_2) 200.0)) _returnvalue_2 (`self.AOERadius`) (`|MakeArray` "ObjectTypeQuery1" "ObjectTypeQuery3" "ObjectTypeQuery2" :!type "EObjectTypeQuery Enum") false (`|MakeArray` (`self.Instigator`) (`self.GetOwner`) :!type "Actor Object Reference") "None" true (struct :`R` 1.0 :`A` 1.0) (struct :`G` 1.0 :`A` 1.0) (`self.DamageTickRate`)))
      (for _array_element _outhits
        (`GameplayStatics.ApplyPointDamage` (`.HitActor` (`GameplayStatics.BreakHitResult` _array_element)) (`self.BaseDamage`) (`self.GetActorForwardVector` (`self.GetOwner`)) _array_element _returnvalue _returnvalue (select `EAbilityDamageType` (`self.DamageType`) :`E_Physical` "/Game/Blueprints/Enumerations/DT_PhysicalDamage.DT_PhysicalDamage_C" :`E_Magical` "/Game/Blueprints/Enumerations/DT_MagicalDamage.DT_MagicalDamage_C" :!type "DamageType Class Reference"))))))

(fn `SetGroundTargeter`
  (params (HitLocation :type "Vector Structure") (HitResult :type "HitResult Structure"))
  (returns (NewParam :type "Vector Structure"))
  (locals (NewLocalVar :type Boolean :default true) (NewLocalVar_0 :type "Vector Structure" :default (0.0 0.0 0.0)) (L_GroundHits :type "Array of HitResult Structure"))
  (bind _l_groundhits (`local.L_GroundHits`))
  (bind (_bblockinghit _binitialoverlap _time _distance _location _impactpoint _normal _impactnormal) (`GameplayStatics.BreakHitResult` (`|GetArrayItem` _l_groundhits)))
  (bind (_returnvalue_roll _returnvalue_pitch) (`KismetMathLibrary.BreakRotator` (`KismetMathLibrary.Conv_VectorToRotator` _impactnormal)))
  (bind _outhits (`KismetSystemLibrary.SphereTraceMultiForObjects` :`Start` (`KismetMathLibrary.MakeVector` (.x HitLocation) (.y HitLocation) (+ (.z HitLocation) 20.0)) :`End` (`KismetMathLibrary.MakeVector` (.x HitLocation) (.y HitLocation) (- (.z HitLocation) 500.0)) :`Radius` 3.0 :`ObjectTypes` (`|MakeArray` "ObjectTypeQuery1" "ObjectTypeQuery2" :!type "EObjectTypeQuery Enum") :`DrawDebugType` "ForOneFrame"))
  (for _array_element _outhits
    (`KismetArrayLibrary.Array_AddUnique` _l_groundhits _array_element)
    (if (`KismetMathLibrary.InRange_FloatFloat` _returnvalue_pitch 30.0 90.0)
      (return _location)
      (else
        (`KismetArrayLibrary.Array_RemoveItem` _l_groundhits _array_element))))
  (`KismetArrayLibrary.Array_Clear` (`local.L_GroundHits`)))

(fn `UserConstructionScript`)