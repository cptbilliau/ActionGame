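; Short-lived basic-attack ability actor for a melee swipe that follows its owner and destroys itself shortly after spawning.
; On BeginPlay it picks and scales the swipe particle from SizeAngle and Range, then fires a fan of multi line traces by stepping an Arrow across that angle.
; HitFunction uses target type and combat-component team to apply damage or healing as point damage, recording affected actors to prevent repeat hits.
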(event `CalculateRotationSteps`
  (set `self.LineCastAmount` (`KismetMathLibrary.FTrunc` (/ (`self.SizeAngle`) (`self.RotationAmount`))))
  (set `self.StartingRotation` (`SceneComponent.K2_GetComponentRotation` (`self.Arrow`)))
  (`SceneComponent.K2_AddWorldRotation` (`self.Arrow`) (`KismetMathLibrary.MakeRotator` 0.0 0.0 (* (/ (`self.SizeAngle`) 2.0) -1.0)) false false))

(event `Destroy`
  (`self.K2_DestroyActor`))

(event `self.ReceiveBeginPlay`
  (`parent.ReceiveBeginPlay`)
  (`self.SetVFXStats`)
  (`ActorComponent.Activate` (`self.ParticleSystem`) true)
  (`|ExecutionSequence`
    (:`then_0`
      (`self.CalculateRotationSteps`)
      (`KismetSystemLibrary.PrintString` (`|GetEnumeratorNameAsString` (`self.AttachedSlot`)))
      (`KismetSystemLibrary.K2_SetTimerDelegate` (delegate `Destroy`) 0.3))
    (:`then_1`
      (for _ (range (+ (`self.LineCastAmount`) 1)) :!label _label
        (bind _outhits (`KismetSystemLibrary.LineTraceMultiForObjects` (`self.K2_GetActorLocation`) (+ (`SceneComponent.K2_GetComponentLocation` (`self.Arrow`)) (* (`KismetMathLibrary.GetForwardVector` (`SceneComponent.K2_GetComponentRotation` (`self.Arrow`))) (`self.Range`))) (`|MakeArray` "ObjectTypeQuery1" "ObjectTypeQuery3" "ObjectTypeQuery2" :!type "EObjectTypeQuery Enum") false (select `EAbilityTargetType` (`self.AbilityTargetType`) :`E_Enemies` (`|MakeArray` (`self.Instigator`) (`self.GetOwner`) :!type "Actor Object Reference")) (`self.Draw Debug Type`) false (struct :`R` 1.0 :`A` 1.0) (struct :`G` 1.0 :`A` 1.0) 2.0))
        (`SceneComponent.K2_AddWorldRotation` (`self.Arrow`) (`KismetMathLibrary.MakeRotator` 0.0 0.0 (`self.RotationAmount`)) false false)
        (`self.HitFunction` _outhits)
        (set `self.NewVar` true))
      (`SceneComponent.K2_SetWorldRotation` (`self.Arrow`) (`self.StartingRotation`) false false)
      (`SceneComponent.K2_AddWorldRotation` (`self.Arrow`) (`KismetMathLibrary.MakeRotator` 0.0 0.0 (* (/ (`self.SizeAngle`) 2.0) -1.0)) false false))))

(event `self.ReceiveTick`
  (params (DeltaSeconds :type "Float (single-precision)"))
  (bind _returnvalue_location (`KismetMathLibrary.BreakTransform` (`self.GetTransform` (`self.GetOwner`))))
  (`self.K2_SetActorLocation` _returnvalue_location)
  (`KismetSystemLibrary.PrintString` "Hello" true true (struct :`G` 0.66 :`B` 1.0 :`A` 1.0) DeltaSeconds)
  (if (`self.NewVar`)
    (goto _label)))

(event `BreakLoop`
  (goto _label :!via `Break`))

(fn `HitFunction`
  (params (Array :type "Array of HitResult Structure"))
  (locals (L_HitActor :type "Actor Object Reference") (L_HitResult :type "HitResult Structure"))
  (bind _returnvalue (`self.GetComponentByClass` (`local.L_HitActor`) "/Game/Blueprints/Components/BP_CombatComponent.BP_CombatComponent_C"))
  (bind _returnvalue_2 (`self.GetComponentByClass` (`local.L_HitActor`) "/Game/Blueprints/Components/BP_CombatComponent.BP_CombatComponent_C"))
  (bind _returnvalue_3 (`self.GetComponentByClass` (`local.L_HitActor`) "/Game/Blueprints/Components/BP_CombatComponent.BP_CombatComponent_C"))
  (for _array_element Array
    (set `local.L_HitResult` _array_element)
    (bind _output_get (set `local.L_HitActor` (`.HitActor` (`GameplayStatics.BreakHitResult` _array_element))))
    (if (not (`KismetArrayLibrary.Array_Contains` (`self.Hit Actors Array`) _output_get))
      (switch `EAbilityTargetType` (`self.AbilityTargetType`)
        (:`E_Enemies`
          (`/Engine/EditorBlueprintResources/StandardMacros.IsValid` _returnvalue_2
            (:`Is Valid`
              ;[1 1 1] Deal Damage
              (if (!= (`CombatComponent.Team` (`self.GetComponentByClass` (`self.Instigator`) "/Game/Blueprints/Components/BP_CombatComponent.BP_CombatComponent_C")) (`CombatComponent.Team` _returnvalue_2)) :!label _label
                (`GameplayStatics.ApplyPointDamage` (`local.L_HitActor`) (`self.GetAbilityDamage`) (`self.K2_GetActorLocation`) (`local.L_HitResult`) (`self.GetInstigatorController`) self (select `EAbilityDamageType` (`self.DamageType`) :`E_Physical` "/Game/Blueprints/Enumerations/DT_PhysicalDamage.DT_PhysicalDamage_C" :`E_Magical` "/Game/Blueprints/Enumerations/DT_MagicalDamage.DT_MagicalDamage_C" :!type "DamageType Class Reference"))
                (`KismetArrayLibrary.Array_AddUnique` (`self.Hit Actors Array`) (`local.L_HitActor`) :!label _label_2)))))
        (:`E_Allies`
          (`/Engine/EditorBlueprintResources/StandardMacros.IsValid` _returnvalue_3
            (:`Is Valid`
              (if (== (`CombatComponent.Team` (`self.GetComponentByClass` (`self.Instigator`) "/Game/Blueprints/Components/BP_CombatComponent.BP_CombatComponent_C")) (`CombatComponent.Team` _returnvalue_3))
                ;[1 1 1] Deal Healing
                (`GameplayStatics.ApplyPointDamage` (`local.L_HitActor`) (`self.GetAbilityHealing`) (`self.K2_GetActorLocation`) (`local.L_HitResult`) (`self.GetInstigatorController`) self "/Game/Blueprints/Enumerations/DT_HealingDamage.DT_HealingDamage_C" :!label _label_3)
                (goto _label_2)
                (else
                  (goto _label))))))
        (:`E_AlliesAndEnemies`
          (`/Engine/EditorBlueprintResources/StandardMacros.IsValid` _returnvalue
            (:`Is Valid`
              (if (== (`CombatComponent.Team` (`self.GetComponentByClass` (`self.Instigator`) "/Game/Blueprints/Components/BP_CombatComponent.BP_CombatComponent_C")) (`CombatComponent.Team` _returnvalue))
                (goto _label_3)
                (else
                  (goto _label))))))))))

(fn `SetVFXStats`
  (bind _sizeangle (`self.SizeAngle`))
  (`|ExecutionSequence`
    (:`then_0`
      ;[1 1 1] Set Width
      (if (>= _sizeangle 150.0)
        (set `self.L_SwipeWidth` 1.1)
        (`ParticleSystemComponent.SetTemplate` (`self.ParticleSystem`) "/Game/VFX/RPGEffects/Particles/P_Warrior_Swipe_WideAngle.P_Warrior_Swipe_WideAngle" :!label _label)
        (elif (>= _sizeangle 120.0)
          (set `self.L_SwipeWidth` 1.0)
          (goto _label)
          (else
            (if (>= _sizeangle 90.0)
              (set `self.L_SwipeWidth` 0.7)
              (else
                (set `self.L_SwipeWidth` 0.35)))
            (`ParticleSystemComponent.SetTemplate` (`self.ParticleSystem`) "/Game/VFX/RPGEffects/Particles/P_Warrior_Swipe_TightAngle.P_Warrior_Swipe_TightAngle")))))
    (:`then_1`
      ;[1 1 1] Set Length
      (if (>= (`self.Range`) 270.0)
        (set `self.L_SwipeLength` 1.25)
        (elif (>= (`self.Range`) 250.0)
          (set `self.L_SwipeLength` 1.15)
          (elif (>= (`self.Range`) 200.0)
            (set `self.L_SwipeLength` 1.05)
            (elif (>= (`self.Range`) 150.0)
              (set `self.L_SwipeLength` 0.7)
              (else
                (set `self.L_SwipeLength` 0.6)))))))
    (:`then_2`
      (`FXSystemComponent.SetVectorParameter` (`self.ParticleSystem`) "Size" (`KismetMathLibrary.MakeVector` (`self.L_SwipeLength`) (`self.L_SwipeWidth`) 1.0)))))

(fn `UserConstructionScript`
  (locals (L_SwipeWidth :type "Float (double-precision)") (L_SwipeLength :type "Float (double-precision)")))