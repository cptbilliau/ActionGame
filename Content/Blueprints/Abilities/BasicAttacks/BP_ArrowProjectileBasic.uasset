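; Basic-attack arrow projectile that reports its slot cooldown to its owner on spawn and expires after its lifetime.
; Construction feeds speed and lifetime into movement and Niagara parameters.
; Capsule overlaps spawn an effect and call HitFunction, which uses combat-component teams to apply damage, or healing as healing-type damage; the Allies mode also damages enemies.
; A separate Hit event deals physical damage without team checks; both destroy the arrow.
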(event `self.ReceiveBeginPlay`
  (`parent.ReceiveBeginPlay`)
  (`KismetSystemLibrary.K2_SetTimerDelegate` (delegate `Destroy`) (`self.Lifetime`))
  (message `/Game/Blueprints/Interfaces/Combat_BPI.SlotFired` (`self.GetOwner`) "E_BasicAttack" (`self.BaseCooldown`)))

(event `Destroy`
  (`self.K2_DestroyActor`))

(event `self.Capsule.OnComponentBeginOverlap`
  (params (OverlappedComponent :type "PrimitiveComponent Object Reference") (OtherActor :type "Actor Object Reference") (OtherComp :type "PrimitiveComponent Object Reference") (OtherBodyIndex :type Integer) (bFromSweep :type Boolean) (SweepResult :type "HitResult Structure (by ref)"))
  (bind (_bblockinghit _binitialoverlap _time _distance _location _impactpoint _normal _impactnormal _physmat _hitactor) (`GameplayStatics.BreakHitResult` SweepResult))
  (`KismetSystemLibrary.PrintString` "hit")
  (if (and (!= _hitactor (`self.GetOwner`)) (!= self _hitactor))
    (`NiagaraFunctionLibrary.SpawnSystemAtLocation` "/Game/sA_Megapack_v1/sA_StylizedAttacksPack/FX/NiagaraSystems/NS_BasicHit_2.NS_BasicHit_2" _location)
    (`self.HitFunction` SweepResult)
    (`self.K2_DestroyActor`)))

(event `self.ReceiveHit`
  (params (MyComp :type "PrimitiveComponent Object Reference") (Other :type "Actor Object Reference") (OtherComp :type "PrimitiveComponent Object Reference") (bSelfMoved :type Boolean) (HitLocation :type "Vector Structure") (HitNormal :type "Vector Structure") (NormalImpulse :type "Vector Structure") (Hit :type "HitResult Structure (by ref)"))
  (bind (_bblockinghit _binitialoverlap _time _distance _location _impactpoint _normal _impactnormal _physmat _hitactor) (`GameplayStatics.BreakHitResult` Hit))
  (`KismetSystemLibrary.PrintString` "hit")
  (if (and (!= _hitactor (`self.GetOwner`)) (!= self _hitactor))
    (`NiagaraFunctionLibrary.SpawnSystemAtLocation` "/Game/Assets/NS_ArcaneHit.NS_ArcaneHit" _location)
    (`GameplayStatics.ApplyPointDamage` _hitactor (`self.GetAbilityDamage`) (`self.GetActorForwardVector` (`self.GetOwner`)) Hit (`self.GetInstigatorController`) self "/Game/Blueprints/Enumerations/DT_PhysicalDamage.DT_PhysicalDamage_C")
    (`self.K2_DestroyActor`)))

(fn `HitFunction`
  (params (Array :type "HitResult Structure"))
  (locals (L_HitActor :type "Actor Object Reference") (L_HitResult :type "HitResult Structure"))
  (bind _returnvalue (`self.GetComponentByClass` (`local.L_HitActor`) "/Game/Blueprints/Components/BP_CombatComponent.BP_CombatComponent_C"))
  (bind _returnvalue_2 (`self.GetComponentByClass` (`local.L_HitActor`) "/Game/Blueprints/Components/BP_CombatComponent.BP_CombatComponent_C"))
  (bind _returnvalue_3 (`self.GetComponentByClass` (`local.L_HitActor`) "/Game/Blueprints/Components/BP_CombatComponent.BP_CombatComponent_C"))
  (bind _output_get (set `local.L_HitResult` Array))
  (set `local.L_HitActor` (`.HitActor` (`GameplayStatics.BreakHitResult` _output_get)))
  (switch `EAbilityTargetType` (`self.AbilityTargetType`)
    (:`E_Enemies`
      (`/Engine/EditorBlueprintResources/StandardMacros.IsValid` _returnvalue_2
        (:`Is Valid`
          (if (!= (`CombatComponent.Team` (`self.GetComponentByClass` (`self.Instigator`) "/Game/Blueprints/Components/BP_CombatComponent.BP_CombatComponent_C")) (`CombatComponent.Team` _returnvalue_2)) :!label _label
            ;[1 1 1] Deal Damage
            (`GameplayStatics.ApplyPointDamage` (`local.L_HitActor`) (`self.GetAbilityDamage`) (`self.K2_GetActorLocation`) (`local.L_HitResult`) (`self.GetInstigatorController`) self (select `EAbilityDamageType` (`self.DamageType`) :`E_Physical` "/Game/Blueprints/Enumerations/DT_PhysicalDamage.DT_PhysicalDamage_C" :`E_Magical` "/Game/Blueprints/Enumerations/DT_MagicalDamage.DT_MagicalDamage_C" :!type "DamageType Class Reference"))))))
    (:`E_Allies`
      (`/Engine/EditorBlueprintResources/StandardMacros.IsValid` _returnvalue_3
        (:`Is Valid`
          (if (== (`CombatComponent.Team` (`self.GetComponentByClass` (`self.Instigator`) "/Game/Blueprints/Components/BP_CombatComponent.BP_CombatComponent_C")) (`CombatComponent.Team` _returnvalue_3))
            ;[1 1 1] Deal Healing
            (`GameplayStatics.ApplyPointDamage` (`local.L_HitActor`) (`self.GetAbilityHealing`) (`self.K2_GetActorLocation`) (`local.L_HitResult`) (`self.GetInstigatorController`) self "/Game/Blueprints/Enumerations/DT_HealingDamage.DT_HealingDamage_C" :!label _label_2)
            (else
              (goto _label))))))
    (:`E_AlliesAndEnemies`
      (`/Engine/EditorBlueprintResources/StandardMacros.IsValid` _returnvalue
        (:`Is Valid`
          (if (== (`CombatComponent.Team` (`self.GetComponentByClass` (`self.Instigator`) "/Game/Blueprints/Components/BP_CombatComponent.BP_CombatComponent_C")) (`CombatComponent.Team` _returnvalue))
            (goto _label_2)
            (else
              (goto _label))))))))

(fn `UserConstructionScript`
  (bind _niagara (`self.Niagara`))
  (set `ProjectileMovementComponent.InitialSpeed` (`self.Speed`) (`self.ProjectileMovement`))
  (`FXSystemComponent.SetVectorParameter` _niagara "Velocity" (`KismetMathLibrary.MakeVector` (`self.Speed`)))
  (`FXSystemComponent.SetFloatParameter` _niagara "Lifetime" (`self.Lifetime`)))