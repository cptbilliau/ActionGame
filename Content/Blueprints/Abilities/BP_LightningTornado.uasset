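; Lightning tornado area-of-effect ability actor that drifts toward a nearby pawn after spawning.
; On BeginPlay it sphere-traces for pawns other than its instigator and stores their impact points.
; If any are hit, GetClosestVector picks the nearest point and MoveComponentTo glides the root there once, without tracking the pawn.
; A timer based on the AOE duration deactivates the particle system one second before that duration ends.
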(event `self.ReceiveBeginPlay`
  (bind _returnvalue (`self.K2_GetActorLocation`))
  (bind (_outhits _returnvalue_2) (`KismetSystemLibrary.SphereTraceMultiForObjects` _returnvalue _returnvalue 500.0 (`|MakeArray` "ObjectTypeQuery3" :!type "EObjectTypeQuery Enum") false (`|MakeArray` (`self.Instigator`) :!type "Actor Object Reference")))
  (for _array_element _outhits
    (`KismetArrayLibrary.Array_Add` (`self.ArrayHitLocations`) (`.ImpactPoint` (`GameplayStatics.BreakHitResult` _array_element))))
  (if _returnvalue_2
    (`self.MoveAbility`))
  (`parent.ReceiveBeginPlay`)
  (`KismetSystemLibrary.K2_SetTimerDelegate` (delegate `CustomEvent`) (- (`self.AOEDuration`) 1.0)))

(event `CustomEvent`
  (`ActorComponent.Deactivate` (`self.ParticleSystem`)))

(event `MoveAbility`
  (`KismetSystemLibrary.MoveComponentTo` (`self.DefaultSceneRoot`) (`self.GetClosestVector` (`self.ArrayHitLocations`)) (struct) false false 4.0))

(fn `GetClosestVector`
  (params (HitPoint :type "Array of Vector Structure"))
  (returns (ClosestPoint :type "Vector Structure"))
  (locals (ClosestDistance :type "Float (double-precision)") (ClosestIndex :type Integer))
  (if (> (`KismetArrayLibrary.Array_Length` (`self.ArrayHitLocations`)) 1)
    (for (_array_element _array_index) HitPoint
      (if (== _array_index 0)
        (bind _returnvalue (`KismetMathLibrary.Vector_Distance` _array_element (`SceneComponent.K2_GetComponentLocation` (`self.DefaultSceneRoot`))))
        (set `local.ClosestDistance` _returnvalue)
        (set `local.ClosestIndex` 0)
        (elif (< _returnvalue (`local.ClosestDistance`))
          (set `local.ClosestDistance` _returnvalue)
          (set `local.ClosestIndex` _array_index))))
    (return (`|GetArrayItem` (`self.ArrayHitLocations`) (`local.ClosestIndex`)))
    (else
      (return (`|GetArrayItem` (`self.ArrayHitLocations`))))))

(fn `UserConstructionScript`
  (`parent.UserConstructionScript`))