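; BP_FireBall is a fireball projectile that explodes on impact and deals magical area damage.
; The construction script passes speed to projectile movement and both speed and lifetime to its Niagara effect.
; A timer destroys it when its lifetime expires.
; Hitting anything but its owner spawns an explosion and sphere-traces the area, applying point damage to each hit except instigator and owner, then destroys the projectile.
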(event `self.ReceiveBeginPlay`
  (`KismetSystemLibrary.K2_SetTimerDelegate` (delegate `Destroy`) (`self.Lifetime`)))

(event `Destroy`
  (`self.K2_DestroyActor`))

(event `self.ReceiveHit`
  (params (MyComp :type "PrimitiveComponent Object Reference") (Other :type "Actor Object Reference") (OtherComp :type "PrimitiveComponent Object Reference") (bSelfMoved :type Boolean) (HitLocation :type "Vector Structure") (HitNormal :type "Vector Structure") (NormalImpulse :type "Vector Structure") (Hit :type "HitResult Structure (by ref)"))
  (bind _returnvalue (`self.GetInstigatorController`))
  (if (not (== (`.HitActor` (`GameplayStatics.BreakHitResult` Hit)) (`self.GetOwner`)))
    (`GameplayStatics.SpawnEmitterAtLocation` "/Game/VFX/FXVarietyPack/Particles/P_ky_explosion.P_ky_explosion" HitLocation (struct) (0.6 0.6 0.6))
    (bind _outhits (`KismetSystemLibrary.SphereTraceMultiForObjects` HitLocation HitLocation 150.0 (`|MakeArray` "ObjectTypeQuery1" "ObjectTypeQuery3" "ObjectTypeQuery2" :!type "EObjectTypeQuery Enum") false (`|MakeArray` (`self.Instigator`) (`self.GetOwner`) :!type "Actor Object Reference")))
    (for _array_element _outhits
      (`GameplayStatics.ApplyPointDamage` (`.HitActor` (`GameplayStatics.BreakHitResult` _array_element)) (`self.BaseDamage`) (`self.GetActorForwardVector` (`self.GetOwner`)) _array_element _returnvalue _returnvalue "/Game/Blueprints/Enumerations/DT_MagicalDamage.DT_MagicalDamage_C"))
    (`self.K2_DestroyActor`)))

(fn `UserConstructionScript`
  (bind _niagara (`self.Niagara`))
  (set `ProjectileMovementComponent.InitialSpeed` (`self.Speed`) (`self.ProjectileMovement`))
  (`FXSystemComponent.SetVectorParameter` _niagara "Velocity" (`KismetMathLibrary.MakeVector` (`self.Speed`)))
  (`FXSystemComponent.SetFloatParameter` _niagara "Lifetime" (`self.Lifetime`)))