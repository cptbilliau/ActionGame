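; BP_ItemComponent is an actor component that makes its owning MasterItem a pickup for the player's inventory.
; On BeginPlay it sets the owner to replicate.
; On interaction it passes the owning item to the player's BPInventoryComponent and destroys the owner if the item is added successfully.
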(event `self.ReceiveBeginPlay`
  (`Actor.SetReplicates` (`self.GetOwner`) true))

(event `/Game/Blueprints/Interfaces/Inventory_BPI.InteractWith`
  (params (`Player Character` :type "/Game/Blueprints/BP_ThirdPersonCharacter Object Reference"))
  (bind _bp_inventorycomponent (`/Game/Blueprints/BP_ThirdPersonCharacter.BP_InventoryComponent` `Player Character`))
  (`/Engine/EditorBlueprintResources/StandardMacros.IsValid` _bp_inventorycomponent
    (:`Is Valid`
      (bind _success (`/Game/Blueprints/Components/BP_InventoryComponent.AddItemToInventory` _bp_inventorycomponent (cast `/Game/Blueprints/Inventory/MasterItem` (`self.GetOwner`) :!pure true)))
      (if _success
        (`Actor.K2_DestroyActor` (`self.GetOwner`))))))