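; Combat component that manages a player's stats, experience, leveling and class-based energy regeneration.
; InitializeStats copies each base value in the stat map to its current value, and Tick uses a Delay to trickle Energy back for Casters only.
; CheckIfShouldLvlUp compares experience against a curve, subtracts the level cost and fires experience and level-up notifications.
; LevelUpFunction raises base stats from the Caster, Warrior or Rogue scaling table.
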(event `self.ReceiveBeginPlay`)

(event `self.ReceiveTick`
  (params (DeltaSeconds :type "Float (single-precision)"))
  (switch `EPlayerClass` (`self.PlayerClass`)
    (:`E_Caster`
      (`KismetSystemLibrary.Delay` 0.1)
      (if (<= (`self.GetCurrentStatValue` "E_Energy") (`self.GetBaseStatValue` "E_Energy"))
        (`self.ModifyCurrentStatValue` "E_Energy" 0.1)))))

(fn `CheckIfShouldLvlUp`
  (params (InExperience :type "Float (double-precision)"))
  (returns (NewParam :type Boolean))
  (if (>= InExperience (`CurveFloat.GetFloatValue` (`self.ExpCurve`) (`KismetMathLibrary.Conv_IntToDouble` (+ (`self.PlayerLevel`) 1))))
    (`KismetSystemLibrary.PrintString` "Leveled UP")
    (`/Engine/EditorBlueprintResources/StandardMacros.IncrementInt` (`self.PlayerLevel`)
      (:`  `
        (bind _output_get (set `self.PlayerExp` (- (`self.PlayerExp`) (`CurveFloat.GetFloatValue` (`self.ExpCurve`) (`KismetMathLibrary.Conv_IntToDouble` (`self.PlayerLevel`))))))
        (`self.OnExperienceGained` _output_get)
        (`KismetSystemLibrary.PrintString` (`KismetStringLibrary.Conv_DoubleToString` 0.0))
        (`self.OnPlayerLevelUp`)
        (return true)))
    (else
      (return false))))

(fn `InitializeStats`
  (bind _keys (`BlueprintMapLibrary.Map_Keys` (`self.PlayerStatMap`)))
  (for _array_element _keys
    (`self.SetCurrentStatValue` _array_element (break `StatStruct` (`BlueprintMapLibrary.Map_Find` (`self.PlayerStatMap`) _array_element)))))

(fn `LevelUpFunction`
  (for _array_element (select `EPlayerClass` (`self.PlayerClass`) :`E_Caster` (`self.CasterLevelScaling`) :`E_Warrior` (`self.WarriorLevelScaling`) :`E_Rogue` (`self.RogueLevelScaling`))
    (`self.ModifyBaseStatValue` (cast `EPlayerStats` (`KismetMathLibrary.Conv_IntToByte` (`KismetMathLibrary.Conv_ByteToInt` (break `ItemStatStruct` _array_element)))) (`.statValue` (break `ItemStatStruct` _array_element)))))