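; Inventory component that holds a character's items in a fixed-size slot array, plus a list of equipped gear.
; Pickups stack by name, auto-equip when their gear slot is free (with one-, two- and either-hand rules), or fill the first empty slot.
; Slot swaps and equipment changes pass through paired Server/Client events.
; MC_Update and equip/unequip dispatchers notify listeners of changes.
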(event `self.ReceiveBeginPlay`
  (`KismetArrayLibrary.Array_Resize` (`self.InventoryArray`) (`self.MaxInventorySize`)))

(event `MC_Update`
  (`self.OnInventoryUpdated`))

(event `Server_TransferSlots`
  (params (`Source Index` :type Integer) (`Source Inventory` :type "/Game/Blueprints/Components/BP_InventoryComponent Object Reference") (`Destination Index` :type Integer))
  (`self.Client Transfer Slots` `Source Index` `Source Inventory` `Destination Index`))

(event `Client Transfer Slots`
  (params (`Source Index` :type Integer) (`Source Inventory` :type "/Game/Blueprints/Components/BP_InventoryComponent Object Reference") (`Destination Index` :type Integer))
  (`self.TransferSlots` `Source Index` `Source Inventory` `Destination Index`))

(event `Server_UnEquip Equipment`
  (params (UnEquippedEquipment :type "/Game/Blueprints/Inventory/EquipmentItemData Structure"))
  (`self.OnEquipmentUnEquipped` UnEquippedEquipment))

(event `Server_Transfer Equipment`
  (params (`Source Index` :type Integer) (`Source Inventory` :type "/Game/Blueprints/Components/BP_InventoryComponent Object Reference") (EquipmentSlotItem :type "/Game/Blueprints/Inventory/EquipmentItemData Structure"))
  (`self.TransferEquipment` `Source Index` `Source Inventory` EquipmentSlotItem))

(event `Client_UnEquip Equipment`
  (params (Equipment :type "/Game/Blueprints/Inventory/EquipmentItemData Structure"))
  (`self.Server_UnEquip Equipment` Equipment))

(event `Client_Transfer Equipment`
  (params (`Source Index` :type Integer) (`Source Inventory` :type "/Game/Blueprints/Components/BP_InventoryComponent Object Reference") (EquipmentSlotItem :type "/Game/Blueprints/Inventory/EquipmentItemData Structure"))
  (`self.Server_Transfer Equipment` `Source Index` `Source Inventory` EquipmentSlotItem))

(event `Client_Equip Equipment`
  (params (Equipment :type "/Game/Blueprints/Inventory/EquipmentItemData Structure"))
  (`self.Server_Equip Equipment` Equipment))

(event `Server_Equip Equipment`
  (params (`Equipment to Equip` :type "/Game/Blueprints/Inventory/EquipmentItemData Structure"))
  (`self.EquipEquipment` `Equipment to Equip`))

(fn `AddItemToInventory`
  (params (ItemIn :type "/Game/Blueprints/Inventory/MasterItem Object Reference"))
  (returns (Success :type Boolean))
  (locals (L_HitItem :type "/Game/Blueprints/Inventory/MasterItem Object Reference") (L_HitEquipment :type "/Game/Blueprints/Inventory/EquipmentItem Object Reference"))
  (bind (_isempty_ _slottoequip) (`self.Is Equipment Slot Empty?` (`local.L_HitItem`)))
  (bind _output_get (set `local.L_HitItem` ItemIn))
  (if (or (`self.Is Equipment Slot Empty?` (`local.L_HitItem`)) (`self.CanAddItem`))
    (if (`/Game/Blueprints/Inventory/MasterItem.GetIsStackable` _output_get)
      (if (`self.HasItemInInventory?` (`/Game/Blueprints/Inventory/MasterItem.GetItemName` (`local.L_HitItem`)))
        (`self.IncreaseItemAmount` (`self.GetItemIndex` (`/Game/Blueprints/Inventory/MasterItem.GetItemName` (`local.L_HitItem`))) (`local.L_HitItem`))
        (return true)
        (else
          (`self.AddNewItemToInventory` (`local.L_HitItem`))
          (return true)))
      (elif _isempty_
        (`KismetSystemLibrary.PrintString` "Add to Equipment")
        (`self.EquipEquipmentFromPickup` (`local.L_HitItem`) _slottoequip)
        (return true)
        (else
          (`KismetSystemLibrary.PrintString` "Add to Inventory")
          (`self.AddNewItemToInventory` (`local.L_HitItem`))
          (return true))))
    (else
      (return false))))

(fn `AddNewItemToInventory`
  (params (`Item to Add` :type "/Game/Blueprints/Inventory/MasterItem Object Reference"))
  (for (_array_element _array_index) (`self.InventoryArray`)
    (if (`KismetStringLibrary.EqualEqual_StrStr` (break `/Game/Blueprints/Inventory/ItemData` (`.ItemData_19_C535DB3948E1DFB4729051A1EE541908` (break `/Game/Blueprints/Inventory/EquipmentItemData` _array_element))))
      (`KismetArrayLibrary.Array_Set` (`self.InventoryArray`) _array_index (`/Game/Blueprints/Inventory/MasterItem.ItemData` `Item to Add`))
      (break))))

(fn `CanAddItem`
  (returns (OutBool :type Boolean))
  (if (<= (`self.CurrentInventorySize`) (- (`self.MaxInventorySize`) 1))
    (`/Engine/EditorBlueprintResources/StandardMacros.IncrementInt` (`self.CurrentInventorySize`)
      (:`  `
        (return true)))
    (else
      (return false))))

(fn `EquipEquipment`
  (params (`Equipment to Equip` :type "/Game/Blueprints/Inventory/EquipmentItemData Structure"))
  (`KismetArrayLibrary.Array_Add` (`self.EquipmentArray`) `Equipment to Equip`)
  (`self.OnEquipmentEquipped` `Equipment to Equip`))

(fn `EquipEquipmentFromPickup`
  (params (ItemToAdd :type "/Game/Blueprints/Inventory/MasterItem Object Reference") (`Slot to Equip` :type "/Game/Blueprints/Enumerations/E_EquipmentSlot Enum" :default "NewEnumerator9"))
  (bind _itemdata (`/Game/Blueprints/Inventory/MasterItem.GetItemData` ItemToAdd))
  (`self.Client_Equip Equipment` _itemdata)
  (`self.OnEquipmentEquippedFromPickUp` _itemdata `Slot to Equip`))

(fn `FindSlot`)

(fn `GetEquipmentArray`
  (returns (Equipment :type "Array of /Game/Blueprints/Inventory/EquipmentItemData Structure"))
  (return (`self.EquipmentArray`)))

(fn `GetInventoryArray`
  (returns (InventoryArray :type "Array of /Game/Blueprints/Inventory/EquipmentItemData Structure"))
  (return (`self.InventoryArray`)))

(fn `GetItemIndex`
  (params (ItemName :type String))
  (returns (Index :type Integer))
  (locals (ItemIndex :type Integer))
  (for (_array_element _array_index) (`self.InventoryArray`)
    (bind _output_get (set `local.ItemIndex` _array_index))
    (if (`KismetStringLibrary.EqualEqual_StrStr` (`local.ItemName`) (break `/Game/Blueprints/Inventory/ItemData` (`.ItemData_19_C535DB3948E1DFB4729051A1EE541908` (break `/Game/Blueprints/Inventory/EquipmentItemData` _array_element))))
      (set `local.ItemIndex` _output_get)
      (break)
      (else
        (set `local.ItemIndex` -1))))
  (return (`local.ItemIndex`)))

(fn `HasItemInInventory?`
  (params (Name :type String))
  (returns (OutBool :type Boolean))
  (locals (HasItem :type Boolean))
  (for _array_element (`self.InventoryArray`)
    (if (`KismetStringLibrary.EqualEqual_StrStr` (break `/Game/Blueprints/Inventory/ItemData` (`.ItemData_19_C535DB3948E1DFB4729051A1EE541908` (break `/Game/Blueprints/Inventory/EquipmentItemData` _array_element))) (`local.Name`))
      (set `local.HasItem` true)
      (`/Engine/EditorBlueprintResources/StandardMacros.DecrementInt` (`self.CurrentInventorySize`)
        (:`  `
          (break)))
      (else
        (set `local.HasItem` false))))
  (return (`local.HasItem`)))

(fn `IncreaseItemAmount`
  (params (Index :type Integer) (HitItem :type "/Game/Blueprints/Inventory/MasterItem Object Reference"))
  (bind _output (`|GetArrayItem` (`self.InventoryArray`) Index))
  (bind (_equipmentstats _equipementlvl _itemrarity _averagestatpercentage _itemdata) (break `/Game/Blueprints/Inventory/EquipmentItemData` _output))
  (bind _structout (setmembers `/Game/Blueprints/Inventory/EquipmentItemData` :`StructRef` _output :`ItemData` (make `/Game/Blueprints/Inventory/ItemData` (break `/Game/Blueprints/Inventory/ItemData` _itemdata) (+ (`.Amount_10_1E37BF4F4EA00B7CB1EC3FB949DD8C1B` (break `/Game/Blueprints/Inventory/ItemData` _itemdata)) (`/Game/Blueprints/Inventory/MasterItem.GetItemAmount` HitItem)) (`.IsStackable_7_7F3981964136D1E5C2B1D0B6A94F1374` (break `/Game/Blueprints/Inventory/ItemData` _itemdata)) (`.ItemImage_16_F6D0A68B49ED23E3CCE90597F0C010CB` (break `/Game/Blueprints/Inventory/ItemData` _itemdata)))))
  (`KismetArrayLibrary.Array_Set` (`self.InventoryArray`) (`local.Index`) _structout))

(fn `Is Equipment Slot Empty?`
  (params (Target :type "/Game/Blueprints/Inventory/MasterItem Object Reference"))
  (returns (`isEmpty?` :type Boolean) (SlotToEquip :type "/Game/Blueprints/Enumerations/E_EquipmentSlot Enum"))
  (locals (L_SlotIsEmpty :type Boolean :default true) (L_TargetItemData :type "/Game/Blueprints/Inventory/EquipmentItemData Structure") (L_OffHandCounter :type Integer))
  (bind _output_get (set `local.L_TargetItemData` (`/Game/Blueprints/Inventory/MasterItem.GetItemData` Target)))
  (switch `/Game/Blueprints/Enumerations/E_EquipmentSlot` (`.EquipmentSlot_22_E887D96C4AB1A8040B4353B5A8EB9540` (break `/Game/Blueprints/Inventory/EquipmentItemData` _output_get))
    (:`NewEnumerator0`
      _)
    (:`NewEnumerator1`
      _)
    (:`NewEnumerator2`
      _)
    (:`NewEnumerator3`
      _)
    (:`NewEnumerator4`
      ;[1 1 1] Main and Off Hand
      (for _array_element (`self.EquipmentArray`) :!label _label
        (bind ((`EquipmentSlot_22_E887D96C4AB1A8040B4353B5A8EB9540` _equipmentslot)) (break `/Game/Blueprints/Inventory/EquipmentItemData` _array_element))
        (if (or (`|EnumEquality` (`.EquipmentSlot_22_E887D96C4AB1A8040B4353B5A8EB9540` (break `/Game/Blueprints/Inventory/EquipmentItemData` (`local.L_TargetItemData`))) _equipmentslot) (`|EnumEquality` "NewEnumerator8" _equipmentslot) (`|EnumEquality` "NewEnumerator5" _equipmentslot))
          (set `local.L_SlotIsEmpty` false)
          (break)
          (else
            (set `local.L_SlotIsEmpty` true))))
      (return (`local.L_SlotIsEmpty`) (`.EquipmentSlot_22_E887D96C4AB1A8040B4353B5A8EB9540` (break `/Game/Blueprints/Inventory/EquipmentItemData` (`local.L_TargetItemData`)))))
    (:`NewEnumerator5`
      (goto _label))
    (:`NewEnumerator6`
      ;[1 1 1] Both Hands
      (for _array_element_2 (`self.EquipmentArray`)
        (bind ((`EquipmentSlot_22_E887D96C4AB1A8040B4353B5A8EB9540` _equipmentslot_2)) (break `/Game/Blueprints/Inventory/EquipmentItemData` _array_element_2))
        (if (`|EnumEquality` "NewEnumerator8" _equipmentslot_2)
          (set `local.L_OffHandCounter` 2)
          (break)
          (elif (or (`|EnumEquality` "NewEnumerator5" _equipmentslot_2) (`|EnumEquality` "NewEnumerator6" _equipmentslot_2) (`|EnumEquality` "NewEnumerator4" _equipmentslot_2))
            (bind _result (`/Engine/EditorBlueprintResources/StandardMacros.IncrementInt` (`local.L_OffHandCounter`))
              (:`  `
                (`KismetSystemLibrary.PrintString` (`KismetStringLibrary.Conv_IntToString` _result)))))))
      (switch `int` (`local.L_OffHandCounter`)
        (:`Default`
          _)
        (:`0`
          (return true "NewEnumerator4"))
        (:`1`
          (return true "NewEnumerator5"))
        (:`2`
          _))
      (return false "NewEnumerator9"))
    (:`NewEnumerator8`
      ;[1 1 1] Two Handed
      (for _array_element_3 (`self.EquipmentArray`)
        (bind ((`EquipmentSlot_22_E887D96C4AB1A8040B4353B5A8EB9540` _equipmentslot_3)) (break `/Game/Blueprints/Inventory/EquipmentItemData` _array_element_3))
        (if (or (`|EnumEquality` "NewEnumerator8" _equipmentslot_3) (`|EnumEquality` "NewEnumerator5" _equipmentslot_3) (`|EnumEquality` "NewEnumerator6" _equipmentslot_3) (`|EnumEquality` "NewEnumerator4" _equipmentslot_3))
          (set `local.L_SlotIsEmpty` false)
          (break)
          (else
            (set `local.L_SlotIsEmpty` true))))
      (return (`local.L_SlotIsEmpty`) "NewEnumerator4"))
    (:`NewEnumerator7`
      (return false "NewEnumerator9")))
  ;[1 1 1] All gear minus rings
  (for _array_element_4 (`self.EquipmentArray`)
    (if (`|EnumEquality` (`.EquipmentSlot_22_E887D96C4AB1A8040B4353B5A8EB9540` (break `/Game/Blueprints/Inventory/EquipmentItemData` (`local.L_TargetItemData`))) (`.EquipmentSlot_22_E887D96C4AB1A8040B4353B5A8EB9540` (break `/Game/Blueprints/Inventory/EquipmentItemData` _array_element_4)))
      (set `local.L_SlotIsEmpty` false)
      (break)
      (else
        (set `local.L_SlotIsEmpty` true))))
  (return (`local.L_SlotIsEmpty`) (`.EquipmentSlot_22_E887D96C4AB1A8040B4353B5A8EB9540` (break `/Game/Blueprints/Inventory/EquipmentItemData` (`local.L_TargetItemData`)))))

(fn `TransferEquipment`
  (params (`Source Index` :type Integer) (`Source Inventory` :type "/Game/Blueprints/Components/BP_InventoryComponent Object Reference") (EquipmentSlotItem :type "/Game/Blueprints/Inventory/EquipmentItemData Structure"))
  (locals (LocalSlotItem :type "/Game/Blueprints/Inventory/EquipmentItemData Structure"))
  (`KismetArrayLibrary.Array_Set` (`/Game/Blueprints/Components/BP_InventoryComponent.InventoryArray` `Source Inventory`) `Source Index` EquipmentSlotItem)
  (`self.Client_UnEquip Equipment` EquipmentSlotItem)
  (bind _returnvalue (`KismetArrayLibrary.Array_RemoveItem` (`self.EquipmentArray`) EquipmentSlotItem))
  (`KismetSystemLibrary.PrintString` (`KismetStringLibrary.Conv_BoolToString` _returnvalue) true true (struct :`R` 0.530794 :`B` 1.0 :`A` 1.0) 8.0)
  (`self.MC_Update`)
  (`self.MC_Update` (`local.Source Inventory`)))

(fn `TransferSlots`
  (params (`Source Index` :type Integer) (`Source Inventory` :type "/Game/Blueprints/Components/BP_InventoryComponent Object Reference") (`Destination Index` :type Integer))
  (locals (LocalSlotItem :type "/Game/Blueprints/Inventory/EquipmentItemData Structure"))
  (set `local.LocalSlotItem` (`|GetArrayItem` (`/Game/Blueprints/Components/BP_InventoryComponent.InventoryArray` `Source Inventory`) `Source Index`))
  (if (not (< `Destination Index` 0))
    (`KismetArrayLibrary.Array_Set` (`/Game/Blueprints/Components/BP_InventoryComponent.InventoryArray` (`local.Source Inventory`)) (`local.Source Index`) (`|GetArrayItem` (`self.InventoryArray`) (`local.Destination Index`)))
    (`KismetArrayLibrary.Array_Set` (`self.InventoryArray`) (`local.Destination Index`) (`local.LocalSlotItem`))
    (`self.MC_Update`)
    (`self.MC_Update` (`local.Source Inventory`))))